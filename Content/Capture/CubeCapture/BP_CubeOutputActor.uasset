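; BP_CubeOutputActor feeds data from a referenced scene cube capture into the material on its Plane mesh.
; On BeginPlay it creates a dynamic material instance from the Plane's first material slot.
; Each tick, while the capture reference is valid, it copies the capture's X, Y and Z values into same-named vector parameters, keeping the material in sync with the capture.
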(event `self.ReceiveTick`
  (params (DeltaSeconds :type "Float (single-precision)"))
  (bind _scenecubecaptureref (`self.SceneCubeCaptureRef`))
  (`/Engine/EditorBlueprintResources/StandardMacros.IsValid` _scenecubecaptureref
    (:`Is Valid`
      (`MaterialInstanceDynamic.SetVectorParameterValue` (stale `self.ReceiveBeginPlay` _returnvalue) "X" (`KismetMathLibrary.Conv_VectorToLinearColor` (`/Game/Blueprints/Character/BP_Character.X` _scenecubecaptureref)))
      (`MaterialInstanceDynamic.SetVectorParameterValue` (stale `self.ReceiveBeginPlay` _returnvalue) "Y" (`KismetMathLibrary.Conv_VectorToLinearColor` (`/Game/Blueprints/Character/BP_Character.Y` _scenecubecaptureref)))
      (`MaterialInstanceDynamic.SetVectorParameterValue` (stale `self.ReceiveBeginPlay` _returnvalue) "Z" (`KismetMathLibrary.Conv_VectorToLinearColor` (`/Game/Blueprints/Character/BP_Character.Z` _scenecubecaptureref))))))

(event `self.ReceiveBeginPlay`
  (bind _plane (`self.Plane`))
  (bind _returnvalue (`PrimitiveComponent.CreateDynamicMaterialInstance` _plane 0 (`PrimitiveComponent.GetMaterial` _plane 0) "None")))

(fn `UserConstructionScript`)