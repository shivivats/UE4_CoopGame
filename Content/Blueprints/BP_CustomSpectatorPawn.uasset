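; BP_CustomSpectatorPawn is a spectator pawn that tracks the orientation of its Camera.
; Each Tick it stores the camera's forward, right and up vectors in the X, Y and Z variables.
; An unconnected debug print would show those vectors as text, and the construction script is empty.
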(event `self.ReceiveTick`
  (params (DeltaSeconds :type "Float (single-precision)"))
  (bind _camera (`self.Camera`))
  (set `self.X` (`SceneComponent.GetForwardVector` _camera))
  (set `self.Y` (`SceneComponent.GetRightVector` _camera))
  (set `self.Z` (`SceneComponent.GetUpVector` _camera)))

(fn `UserConstructionScript`)