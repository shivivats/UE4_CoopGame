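; Player character Blueprint that sets up the local player's HUD.
; On BeginPlay, a locally controlled instance creates crosshair, health indicator and ammo widgets and adds them to the viewport.
; Key 1 toggles a random-movement flag, but its branch is unconnected and RandomMovementScript is empty.
; A spectate event only prints a test string, and an eye-direction debug line is left unwired.
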(event `self.ReceiveBeginPlay`
  (if (`self.IsLocallyControlled`)
    (`|ExecutionSequence`
      (:`then_0`
        (bind _returnvalue (`|CreateWidget` "/Game/UserInterface/Widgets/WBP_Crosshair.WBP_Crosshair_C"))
        (`UserWidget.AddToViewport` _returnvalue 0))
      (:`then_1`
        (bind _returnvalue_2 (`|CreateWidget` "/Game/UserInterface/Widgets/WBP_HealthIndicator.WBP_HealthIndicator_C"))
        (`UserWidget.AddToViewport` _returnvalue_2 0))
      (:`then_2`
        (bind _returnvalue_3 (`|CreateWidget` "/Game/UserInterface/Widgets/WBP_AmmoHud.WBP_AmmoHud_C"))
        (`UserWidget.AddToViewport` _returnvalue_3 0)))))

(event `Temp_IsBeingSpectated`
  (`KismetSystemLibrary.PrintString` "Hello"))

(event `self.ReceiveTick`
  (params (DeltaSeconds :type "Float (single-precision)")))

(event `Key|One`
  (params (Key :type "Key Structure"))
  (:`Pressed`
    (set `self.bShouldRandomMove` (not (`self.bShouldRandomMove`)))))

(fn `RandomMovementScript`)

(fn `UserConstructionScript`)