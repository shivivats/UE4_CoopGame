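; Player controller that forwards a debug key press to the test game mode.
; Pressing 1 casts the game mode to BP_TestGameMode and calls IdkPlayerDoStuff.
; Disconnected leftover chains would start, stop and replay recordings through SReplayGameInstance with debug prints, but nothing triggers them.
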(event `Key|One`
  (params (Key :type "Key Structure"))
  (:`Pressed`
    (bind _asbp_test_game_mode (cast `/Game/Blueprints/BP_TestGameMode` (`GameplayStatics.GetGameMode`)))
    (`/Game/Blueprints/BP_TestGameMode.IdkPlayerDoStuff` _asbp_test_game_mode)))

(event `Key|Two`
  (params (Key :type "Key Structure")))

(event `Key|Three`
  (params (Key :type "Key Structure")))

(fn `UserConstructionScript`)