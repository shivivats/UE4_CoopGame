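; BP_GrenadeProjectile is a timed grenade actor that explodes shortly after spawning, with no impact trigger in its graph.
; After a short delay on BeginPlay, it spawns an explosion particle and applies radial damage within ExplosionRadius, credited to the owner's instigator controller.
; It also draws a debug sphere showing the blast radius, then destroys itself.
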(event `self.ReceiveBeginPlay`
  (bind _returnvalue (`self.K2_GetActorLocation`))
  (bind _explosionradius (`self.ExplosionRadius`))
  (`KismetSystemLibrary.Delay` 1.0)
  (`GameplayStatics.SpawnEmitterAtLocation` "/Game/WeaponEffects/Explosion/P_Explosion.P_Explosion" _returnvalue)
  (`GameplayStatics.ApplyRadialDamage` :`BaseDamage` 20.0 :`Origin` _returnvalue :`DamageRadius` _explosionradius :`DamageTypeClass` (`self.DamageType`) :`DamageCauser` self :`InstigatedByController` (`self.GetInstigatorController` (`self.GetOwner`)) :`DamagePreventionChannel` "ECC_WorldStatic")
  (`KismetSystemLibrary.DrawDebugSphere` _returnvalue _explosionradius 12 (struct :`R` 1.0 :`G` 0.949909 :`B` 0.006095 :`A` 1.0) 1.0 1.0)
  (`self.K2_DestroyActor`))

(fn `UserConstructionScript`)