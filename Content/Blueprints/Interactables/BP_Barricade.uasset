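; Interactable barricade that players can place and remove by toggling it on each interaction.
; A FlipFlop on the interaction component's OnInteract event drives the barricade mesh's visibility and collision together.
; It also switches the prompt between "Barricade" and "Remove Barricade", passing the text to MulticastInteract, which sets it again.
; Only the prompt text goes through that event; mesh changes are applied directly in OnInteract.
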(event `self.InteractionComp.OnInteract`
  (params (Character :type "SCharacter Object Reference"))
  (bind _barricademesh (`self.BarricadeMesh`))
  (bind _isa (`/Engine/EditorBlueprintResources/StandardMacros.FlipFlop`)
    (:`A`
      _)
    (:`B`
      _))
  (`SceneComponent.SetVisibility` _barricademesh _isa false)
  (if _isa
    (`PrimitiveComponent.SetCollisionEnabled` _barricademesh "QueryAndPhysics")
    (else
      (`PrimitiveComponent.SetCollisionEnabled` _barricademesh "NoCollision")))
  (bind _returnvalue (select `bool` _isa :`false` "Barricade" :`true` "Remove Barricade"))
  (`SInteractionComponent.SetInteractableActionText` (`self.InteractionComp`) _returnvalue)
  (`self.MulticastInteract` _returnvalue))

(event `MulticastInteract`
  (params (NewActionText :type Text))
  (`SInteractionComponent.SetInteractableActionText` (`self.InteractionComp`) NewActionText))

(fn `UserConstructionScript`)