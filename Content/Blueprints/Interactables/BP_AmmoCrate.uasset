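; BP_AmmoCrate is an interactable crate that adds ammo to the interacting character's current weapon, with a limited number of resupplies.
; Interaction proceeds only while resupplies remain, the character's controller is not local and the current weapon is valid.
; Each use decrements the count and passes it to a multicast event that updates NumResupplies.
; Tick draws the remaining count as debug text at the interaction component.
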(event `self.ReceiveTick`
  (params (DeltaSeconds :type "Float (single-precision)"))
  (`KismetSystemLibrary.DrawDebugString` (`SceneComponent.K2_GetComponentLocation` (`self.InteractionComp`)) (`KismetStringLibrary.Conv_IntToString` (`self.NumResupplies`)) null (struct :`R` 1.0 :`G` 0.024497 :`B` 0.134169 :`A` 1.0)))

(event `self.InteractionComp.OnInteract`
  (params (Character :type "SCharacter Object Reference"))
  (bind _currentweapon (`SCharacter.CurrentWeapon` Character))
  (if (> (`self.NumResupplies`) 0)
    (if (not (`Controller.IsLocalController` (`Pawn.GetController` Character)))
      (`/Engine/EditorBlueprintResources/StandardMacros.IsValid` _currentweapon
        (:`Is Valid`
          (`SWeapon.AddAmmo` _currentweapon)
          (bind _output_get (set `self.NumResupplies` (- (`self.NumResupplies`) 1)))
          (`self.MulticastAmmoCrateResupplyCount` _output_get))))))

(event `MulticastAmmoCrateResupplyCount`
  (params (NewResupplyCount :type Integer))
  (set `self.NumResupplies` NewResupplyCount))

(fn `UserConstructionScript`)