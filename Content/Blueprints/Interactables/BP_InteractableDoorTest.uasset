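; Test interactable door that toggles a barricade on and off when the player interacts with it.
; On each SInteraction OnInteract event, a FlipFlop drives the Door component's visibility and switches its collision between query-and-physics and none.
; The same state sets the interaction prompt text to either "Remove Barricade" or "Barricade".
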(event `self.SInteraction.OnInteract`
  (params (Character :type "SCharacter Object Reference"))
  (bind _door (`self.Door`))
  (bind _isa (`/Engine/EditorBlueprintResources/StandardMacros.FlipFlop`)
    (:`A`
      _)
    (:`B`
      _))
  (`SceneComponent.SetVisibility` _door _isa false)
  (if _isa
    (`PrimitiveComponent.SetCollisionEnabled` _door "QueryAndPhysics")
    (else
      (`PrimitiveComponent.SetCollisionEnabled` _door "NoCollision")))
  (`SInteractionComponent.SetInteractableActionText` (`self.SInteraction`) (select `bool` _isa :`false` "Barricade" :`true` "Remove Barricade")))

(fn `UserConstructionScript`)