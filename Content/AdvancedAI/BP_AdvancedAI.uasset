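; BP_AdvancedAI is an AI-controlled pawn driven by the BT_AdvancedAI behavior tree.
; On BeginPlay, only the authority tells the pawn's AI controller to run that tree.
; Every Tick it draws the HealthComp health value as green debug text at the spring arm's world location.
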(event `self.ReceiveBeginPlay`
  (if (`self.HasAuthority`)
    (`AIController.RunBehaviorTree` (`AIBlueprintHelperLibrary.GetAIController` self) "/Game/AdvancedAI/BT_AdvancedAI.BT_AdvancedAI")))

(event `self.ReceiveTick`
  (params (DeltaSeconds :type "Float (single-precision)"))
  (`KismetSystemLibrary.DrawDebugString` (`SceneComponent.K2_GetComponentLocation` (`self.SpringArmComp`)) (`KismetStringLibrary.Conv_DoubleToString` (`SHealthComponent.Health` (`self.HealthComp`))) null (struct :`R` 0.049283 :`G` 1.0 :`B` 0.08844 :`A` 1.0)))

(fn `UserConstructionScript`)